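; Data recorder that logs the player camera's transform to a CSV file in the project directory when play ends.
; Tick uses a Delay to sample the first found Pawn's camera at roughly FrameRate, buffering one numbered text row per sample.
; Rows hold position divided by 100, plus up and right vectors with Y and Z swapped.
; Rotation-to-quaternion helpers exist but are not used in the recording path.
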(event EventBeginPlay)

(event EventTick
  (params (DeltaSeconds :type Float%20%28single-precision%29))
  ;[1 1 1] Feed Data Buffer
  (Utilities|FlowControl|Delay (/ 1.0 (Variables|Default|GetFrameRate)))
  (bind _outactors (Actor|GetAllActorsOfClass "/Script/Engine.Pawn"))
  (Variables|Default|SetFrameNum (+ (Variables|Default|GetFrameNum) 1))
  (bind _array (CallFunction|CollectTransformtoArray (Transformation|GetWorldLocation (Actor|GetComponentbyClass (Utilities|Array|Get(acopy) _outactors) "/Script/Engine.CameraComponent")) (Math|Vector|GetUpVector (Actor|GetComponentbyClass (Utilities|Array|Get(acopy) _outactors) "/Script/Engine.CameraComponent")) (Math|Vector|GetRightVector (Actor|GetComponentbyClass (Utilities|Array|Get(acopy) _outactors) "/Script/Engine.CameraComponent"))))
  (Utilities|Array|AppendArray (Variables|Default|GetFileText) _array))

(event EventEndPlay
  (params (EndPlayReason :type EEndPlayReason%20Enum :default "Destroyed"))
  ;[1 1 1] Save CSV file
  (Class|RWTxtFile|SaveArrayText (Class|KismetSystemLibrary|GetProjectDirectory) (Utilities|String|Append (Variables|Default|GetFileName) ".csv") (Variables|Default|GetFileText) false))

(fn ConstructionScript)

(fn CollectTransformtoArray
  (params (Pos :type Vector) (Up :type Vector) (Right :type Vector))
  (bind _returnvalue (CallFunction|AppendPos Pos (Utilities|String|Append (Variables|Default|GetBuffer) (Utilities|String|ToString(Integer) (Variables|Default|GetFrameNum)) ",")))
  (bind _newparam (CallFunction|AppendVector Up _returnvalue))
  (bind _newparam_2 (CallFunction|AppendVector Right _newparam))
  (return (Utilities|Array|MakeArray _newparam_2)))

(fn RotatortoQuaternion
  (params (roll :type Float%20%28single-precision%29) (pitch :type Float%20%28single-precision%29) (yaw :type Float%20%28single-precision%29))
  (bind _returnvalue (* roll 0.5))
  (bind _returnvalue_2 (* pitch 0.5))
  (bind _returnvalue_3 (* yaw 0.5))
  (bind _returnvalue_4 (Math|Trig|Cos(Degrees) _returnvalue))
  (bind _returnvalue_5 (Math|Trig|Sin(Degrees) _returnvalue))
  (bind _returnvalue_6 (Math|Trig|Cos(Degrees) _returnvalue_2))
  (bind _returnvalue_7 (Math|Trig|Sin(Radians) _returnvalue_2))
  (bind _returnvalue_8 (Math|Trig|Cos(Degrees) _returnvalue_3))
  (bind _returnvalue_9 (Math|Trig|Sin(Radians) _returnvalue_3))
  (return (+ (* _returnvalue_4 _returnvalue_6 _returnvalue_8) (* _returnvalue_5 _returnvalue_7 _returnvalue_9)) (- (* _returnvalue_4 _returnvalue_6 _returnvalue_9) (* _returnvalue_5 _returnvalue_7 _returnvalue_8)) (+ (* _returnvalue_5 _returnvalue_6 _returnvalue_9) (* _returnvalue_4 _returnvalue_7 _returnvalue_8)) (- (* _returnvalue_5 _returnvalue_6 _returnvalue_8) (* _returnvalue_4 _returnvalue_7 _returnvalue_9))))

(fn AppendPos
  (params (Pos :type Vector) (Text :type String))
  (return (Utilities|String|Append (Utilities|String|Append (Utilities|String|Append Text (Utilities|String|ToString(Float) (/ (.x Pos) 1e+02)) ",") (Utilities|String|ToString(Float) (/ (.y Pos) 1e+02)) ",") (Utilities|String|ToString(Float) (/ (.z Pos) 1e+02)) ",")))

(fn AppendRot
  (params (Rotaion :type Rotator) (Text :type String))
  (bind _returnvalue (Class|KismetMathLibrary|ToQuaterion(Vector) (Math|Vector|MakeVector (.roll Rotaion) (.pitch Rotaion) (.yaw Rotaion))))
  (return (Utilities|String|Append (Utilities|String|Append (Utilities|String|Append (Utilities|String|Append Text (Utilities|String|ToString(Float) (.x _returnvalue)) ",") (Utilities|String|ToString(Float) (.z _returnvalue)) ",") (Utilities|String|ToString(Float) (.y _returnvalue)) ",") (Utilities|String|ToString(Float) (.w _returnvalue)) ",")))

(fn AppendVector
  (params (InFloat :type Vector) (Text :type String))
  (return (Utilities|String|Append (Utilities|String|Append (Utilities|String|Append Text (Utilities|String|ToString(Float) (.x InFloat)) ",") (Utilities|String|ToString(Float) (.z InFloat)) ",") (Utilities|String|ToString(Float) (.y InFloat)) ",")))