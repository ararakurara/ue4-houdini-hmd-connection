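; BP_DataActor records the camera motion of the first pawn found in the level and exports it as CSV.
; Tick passes through a Delay set by FrameRate, then appends a numbered row of camera position and rotation to FileText.
; Position is converted to meters with Y and Z swapped, and rotation is written as roll, pitch, yaw.
; EndPlay saves the buffered rows to a named CSV file in the project directory.
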(event EventBeginPlay
  (Development|PrintString "Hello"))

(event EventTick
  (params (DeltaSeconds :type Float%20%28single-precision%29))
  ;[1 1 1] Feed Data Buffer
  (Utilities|FlowControl|Delay (/ 1.0 (Variables|Default|GetFrameRate)))
  (bind _outactors (Actor|GetAllActorsOfClass "/Script/Engine.Pawn"))
  (Variables|Default|SetFrameNum (+ (Variables|Default|GetFrameNum) 1))
  (Utilities|Array|AppendArray (Variables|Default|GetFileText) (Utilities|Array|MakeArray (Utilities|String|Append (Utilities|String|Append (Utilities|String|Append (Utilities|String|Append (Utilities|String|Append (Utilities|String|Append (Utilities|String|Append (Variables|Default|GetBuffer) (Utilities|String|ToString(Integer) (Variables|Default|GetFrameNum)) ",") (Utilities|String|ToString(Float) (/ (.x (.location (Transformation|GetWorldTransform (Actor|GetComponentbyClass (Utilities|Array|Get(acopy) _outactors) "/Script/Engine.CameraComponent")))) 1e+02)) ",") (Utilities|String|ToString(Float) (/ (.z (.location (Transformation|GetWorldTransform (Actor|GetComponentbyClass (Utilities|Array|Get(acopy) _outactors) "/Script/Engine.CameraComponent")))) 1e+02)) ",") (Utilities|String|ToString(Float) (/ (.y (.location (Transformation|GetWorldTransform (Actor|GetComponentbyClass (Utilities|Array|Get(acopy) _outactors) "/Script/Engine.CameraComponent")))) 1e+02)) ",") (Utilities|String|ToString(Float) (.roll (.rotation (Transformation|GetWorldTransform (Actor|GetComponentbyClass (Utilities|Array|Get(acopy) _outactors) "/Script/Engine.CameraComponent"))))) ",") (Utilities|String|ToString(Float) (.pitch (.rotation (Transformation|GetWorldTransform (Actor|GetComponentbyClass (Utilities|Array|Get(acopy) _outactors) "/Script/Engine.CameraComponent"))))) ",") (Utilities|String|ToString(Float) (.yaw (.rotation (Transformation|GetWorldTransform (Actor|GetComponentbyClass (Utilities|Array|Get(acopy) _outactors) "/Script/Engine.CameraComponent")))))))))

(event EventEndPlay
  (params (EndPlayReason :type EEndPlayReason%20Enum :default "Destroyed"))
  ;[1 1 1] Save CSV file
  (Class|RWTxtFile|SaveArrayText (Class|KismetSystemLibrary|GetProjectDirectory) (Utilities|String|Append (Variables|Default|GetFileName) ".csv") (Variables|Default|GetFileText) false))

(fn ConstructionScript)